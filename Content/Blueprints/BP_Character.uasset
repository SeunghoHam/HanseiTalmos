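; Player character Blueprint with an aimed, slow-motion teleport on Space.
; Holding Space shows the mesh, shifts the camera by timeline, slows time, then moves a spawned target via camera line traces in a RetriggerableDelay loop.
; Release restores time, lerps the actor to the target with an FOV kick and reverses the camera shift.
; Shooting only prints debug text; zoom is unfinished, with disconnected timelines and an uncalled CameraChange.
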(event `self.ReceiveBeginPlay`
  (`SceneComponent.SetVisibility` (`self.Mesh`) false false))

(event `InputAction|Space`
  (params (Key :type "Key Structure"))
  (bind _tptargetpointref (`self.tpTargetPointRef`))
  (bind _mesh (`self.Mesh`))
  (bind _normalcamera (`self.NormalCamera`))
  (bind _returnvalue (`SceneComponent.K2_GetComponentLocation` _normalcamera))
  (:`Pressed`
    (`SceneComponent.SetVisibility` _mesh true false)
    (if (`self.canTeleport?`)
      (bind (_direction _camerashiftspeed) (`Timeline|CameraShift` :!via `PlayFromStart`)
        (:`Update`
          (`SceneComponent.K2_SetRelativeLocationAndRotation` (`self.NormalCamera`) (`KismetMathLibrary.VLerp` (`self.CameraPlayLocation`) (`self.TeleportCamLocation`) _camerashiftspeed) (`KismetMathLibrary.RLerp` (struct) (`self.TeleportCameraRotation`) _camerashiftspeed true) false false))
        (:`Finished`
          (`GameplayStatics.SetGlobalTimeDilation` 0.25)
          (bind _returnvalue_2 (`|SpawnActorFromClass` "/Game/Blueprints/Teleport/TeleportTarget.TeleportTarget_C" (`SceneComponent.K2_GetComponentToWorld` (`self.Scene`)) "Undefined" "OverrideRootScale" null null))
          (set `self.tpTargetPointRef` _returnvalue_2)
          (bind _output_get (set `self.Teleporting` true))
          (if _output_get :!label _label
            (bind _outhit (`KismetSystemLibrary.LineTraceSingle` _returnvalue (+ _returnvalue (* (`SceneComponent.GetForwardVector` _normalcamera) (`self.TeleportRange`))) "TraceTypeQuery1"))
            (bind (_bblockinghit _binitialoverlap _time _distance _location) (`GameplayStatics.BreakHitResult` _outhit))
            (if _bblockinghit
              (`self.K2_SetActorLocation` (`self.tpTargetPointRef`) _location false false))
            (`KismetSystemLibrary.RetriggerableDelay` 0.01)
            (goto _label))))))
  (:`Released`
    (`SceneComponent.SetVisibility` _mesh false false)
    (if (`self.Teleporting`)
      (set `self.Teleporting` false)
      (`GameplayStatics.SetGlobalTimeDilation` 1.0)
      (`/Engine/EditorBlueprintResources/StandardMacros.IsValid` _tptargetpointref
        (:`Is Valid`
          (set `self.TeleportLocation` (`self.K2_GetActorLocation` _tptargetpointref))
          (`self.K2_DestroyActor` _tptargetpointref)
          (`|ExecutionSequence`
            (:`then_0`
              (bind (_direction_2 _teleportspeed) (`Timeline|TeleportSpeed` :!via `PlayFromStart`)
                (:`Update`
                  ;[1 1 1] 텔레포트!
                  (`self.K2_SetActorLocation` (`KismetMathLibrary.VLerp` (`self.K2_GetActorLocation` self) (+ (`self.TeleportLocation`) (0.0 0.0 90.0)) _teleportspeed))
                  ;[1 1 1] 텔레포트 시야각
                  (set `CameraComponent.FieldOfView` (`KismetMathLibrary.Lerp` 120.0 90.0 _teleportspeed) (`self.NormalCamera`)))))
            (:`then_1`
              (bind (_direction_3 _camerashiftspeed_2) (`Timeline|타임라인_0` :!via `ReverseFromEnd`)
                (:`Update`
                  (`SceneComponent.K2_SetRelativeLocationAndRotation` (`self.NormalCamera`) (`KismetMathLibrary.VLerp` (`self.CameraPlayLocation`) (`self.TeleportCamLocation`) _camerashiftspeed_2) (`KismetMathLibrary.RLerp` (struct) (`self.TeleportCameraRotation`) _camerashiftspeed_2 true) false false))))))))))

(event `self.ReceiveTick`
  (params (DeltaSeconds :type "Float (single-precision)")))

(event `self.OnPressed_l_button`
  (if (`self.Zoom`)
    (`KismetSystemLibrary.PrintString` "줌상태 슛" true true (struct :`G` 0.66 :`B` 1.0 :`A` 1.0) 0.5)
    (else
      (`KismetSystemLibrary.PrintString` "노줌 슛" true true (struct :`G` 0.66 :`B` 1.0 :`A` 1.0) 0.5))))

(event `self.OnPressed_r_Button`
  ;[1 1 1] Zoom / Normal StateChnage
)

(event `self.OnReleased_r_Button`
  ;[1 1 1] Zoom / Normal StateChnage
)

(fn `CameraChange`
  (bind _normalcamera (`self.NormalCamera`))
  (bind _zoomcamera (`self.ZoomCamera`))
  (if (`self.Zoom`)
    (`ActorComponent.SetActive` _normalcamera false false)
    (`ActorComponent.SetActive` _zoomcamera true false)
    (else
      (`ActorComponent.SetActive` _normalcamera true false)
      (`ActorComponent.SetActive` _zoomcamera true false))))

(fn `UserConstructionScript`)