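; BP_PC is a player controller that owns the player's HUD and build menu input.
; On BeginPlay it creates the HeadsUpDisplay widget, stores it and adds it to the viewport.
; The Menu input action toggles the build menu through the widget, then uses the returned visibility to switch between Game and UI input with a cursor and game-only input without one.
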(event `self.ReceiveBeginPlay`
  (bind _returnvalue (`|CreateWidget` "/Game/Blueprints/widget/Build/HeadsUpDisplay.HeadsUpDisplay_C"))
  (bind _output_get (set `self.HeadsUpDisplay` _returnvalue))
  (`UserWidget.AddToViewport` _output_get 0))

(event `InputAction|Menu`
  (params (Key :type "Key Structure"))
  (:`Pressed`
    (bind _returnvalue (`/Game/Blueprints/widget/Build/HeadsUpDisplay.ToggleBuildMenu` (`self.HeadsUpDisplay`)))
    (switch `ESlateVisibility` _returnvalue
      (:`Visible`
        (`WidgetBlueprintLibrary.SetInputMode_GameAndUIEx` self null)
        (set `self.bShowMouseCursor` true))
      (:`Hidden`
        (`WidgetBlueprintLibrary.SetInputMode_GameOnly` self)
        (set `self.bShowMouseCursor` false)))))

(fn `UserConstructionScript`)